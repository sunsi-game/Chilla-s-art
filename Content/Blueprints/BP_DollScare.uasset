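; BP_DollScare is a one-shot doll jump scare that the player triggers by interacting while inside its Box trigger.
; The first valid interaction damages the player, plays the Baby sound and starts the TL_Scare timeline.
; The timeline scales the doll toward TargetScale and, after a short Delay, applies a yaw shake.
; The shake offsets from OriginalRotation, which this graph never sets, unlike OriginalScale, which is cached at BeginPlay.
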(event `self.Box.OnComponentBeginOverlap`
  (params (OverlappedComponent :type "PrimitiveComponent Object Reference") (OtherActor :type "Actor Object Reference") (OtherComp :type "PrimitiveComponent Object Reference") (OtherBodyIndex :type Integer) (bFromSweep :type Boolean) (SweepResult :type "HitResult Structure (by ref)"))
  ;[0.07535 0.15 0.09974 0.5] Box Overlap
  (cast `/Game/Horror_Template/Blueprinnts/BP_ThirdPersonCharacter` OtherActor)
  (set `self.bPlayerinRange` true))

(event `self.ReceiveBeginPlay`
  ;[0.038 0.09089 0.15 0.5] BeginPlay
  (set `self.OriginalScale` (`self.GetActorScale3D`)))

(event `self.Box.OnComponentEndOverlap`
  (params (OverlappedComponent :type "PrimitiveComponent Object Reference") (OtherActor :type "Actor Object Reference") (OtherComp :type "PrimitiveComponent Object Reference") (OtherBodyIndex :type Integer))
  ;[0.07535 0.15 0.09974 0.5] Box Overlap
  (cast `/Game/Horror_Template/Blueprinnts/BP_ThirdPersonCharacter` OtherActor)
  (set `self.bPlayerinRange` false))

(event `/Game/Horror_Template/Blueprinnts/Interfaces/Interaction_Interface/BPI_Interaction.Interaction`
  (if (`self.bPlayerinRange`)
    (`self.StartScare`)))

(event `StartScare`
  (if (not (`self.Is one??`))
    (set `self.Is one??` true)
    (if (not (`self.bTriggered`))
      (set `self.bTriggered` true)
      (`GameplayStatics.ApplyDamage` (`GameplayStatics.GetPlayerCharacter` 0) (`self.DamageAmount`) (`GameplayStatics.GetPlayerController` 0) self "/Script/Engine.DamageType")
      (`GameplayStatics.PlaySoundAtLocation` "/Game/BP_Level/Sounds/baby.baby" (`self.K2_GetActorLocation`) (struct) 1.4 1.0 0.0 null null null null)
      (bind (_direction _scalealpha _shakealpha) (`Timeline|TL_Scare`)
        (:`Update`
          (`self.SetActorScale3D` (`KismetMathLibrary.VLerp` (`self.OriginalScale`) (`self.TargetScale`) _scalealpha))
          (`KismetSystemLibrary.Delay` 0.2)
          (`self.K2_SetActorRotation` (`KismetMathLibrary.MakeRotator` 0.0 0.0 (+ (.yaw (`self.Original Rotation`)) (* _shakealpha 10.0)))))))))

(fn `UserConstructionScript`)