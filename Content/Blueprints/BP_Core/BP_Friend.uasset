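; BP_Friend is a story trigger that plays a voiced monologue when the player gets no answer and decides to hurry to school.
; Overlapping its Box as BP_ThirdPersonCharacter sends two timed, input-blocking Korean lines to BP_MessageDirector, found through GetActorOfClass.
; After the delays, it hides the referenced IsHidePush actor, disables its mesh collision and turns off the IsRanton point light.
; The overlap has no one-shot guard.
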(event `self.Box.OnComponentBeginOverlap`
  (params (OverlappedComponent :type "PrimitiveComponent Object Reference") (OtherActor :type "Actor Object Reference") (OtherComp :type "PrimitiveComponent Object Reference") (OtherBodyIndex :type Integer) (bFromSweep :type Boolean) (SweepResult :type "HitResult Structure (by ref)"))
  (cast `/Game/Horror_Template/Blueprinnts/BP_ThirdPersonCharacter` OtherActor)
  (bind _returnvalue (`GameplayStatics.GetActorOfClass` "/Game/BP_Level/UI/BP_MessageDirector.BP_MessageDirector_C"))
  (`/Game/BP_Level/UI/BP_MessageDirector.PlayMessageWithVoice` _returnvalue "실례합니다.." "/Game/BP_Level/Voices/hiん。.hiん。" true)
  (`KismetSystemLibrary.Delay` 2.5)
  (bind _returnvalue_2 (`GameplayStatics.GetActorOfClass` "/Game/BP_Level/UI/BP_MessageDirector.BP_MessageDirector_C"))
  (`/Game/BP_Level/UI/BP_MessageDirector.PlayMessageWithVoice` _returnvalue_2 "대답이 없어… 빨리 학교에 가봐야겠어……" "/Game/BP_Level/Voices/school.school" true)
  (`KismetSystemLibrary.Delay` 5.0)
  (`self.SetActorHiddenInGame` (`self.isHidePush`) true)
  (`PrimitiveComponent.SetCollisionEnabled` (`StaticMeshActor.StaticMeshComponent` (`self.isHidePush`)) "NoCollision")
  (`LightComponent.SetIntensity` (`PointLight.PointLightComponent` (`self.isRanton`)) 0.0))

(fn `UserConstructionScript`)