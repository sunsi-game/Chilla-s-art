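; BP_KeypadPanel is an interactable keypad that opens its linked door when the player enters the correct code.
; An interaction box tracks whether the player character is in range, and Interaction then opens a keypad widget with UI-only input and character input disabled.
; The widget gets a reference back to the panel, which handles digit entry up to four characters, clearing and submission.
; A wrong code briefly shows an error, then resets.
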(event `self.ReceiveBeginPlay`)

(event `/Game/Horror_Template/Blueprinnts/Interfaces/Interaction_Interface/BPI_Interaction.Interaction`
  (if (`self.bPlayerInRange`)
    (`self.OpenKeypadUI`)))

(event `self.InteractionBox.OnComponentBeginOverlap`
  (params (OverlappedComponent :type "PrimitiveComponent Object Reference") (OtherActor :type "Actor Object Reference") (OtherComp :type "PrimitiveComponent Object Reference") (OtherBodyIndex :type Integer) (bFromSweep :type Boolean) (SweepResult :type "HitResult Structure (by ref)"))
  ;[0.05428 0.1446 0.15 0.5] Overlap
  (cast `/Game/Horror_Template/Blueprinnts/BP_ThirdPersonCharacter` OtherActor)
  (set `self.bPlayerInRange` true))

(event `self.InteractionBox.OnComponentEndOverlap`
  (params (OverlappedComponent :type "PrimitiveComponent Object Reference") (OtherActor :type "Actor Object Reference") (OtherComp :type "PrimitiveComponent Object Reference") (OtherBodyIndex :type Integer))
  ;[0.05428 0.1446 0.15 0.5] Overlap
  (cast `/Game/Horror_Template/Blueprinnts/BP_ThirdPersonCharacter` OtherActor)
  (set `self.bPlayerInRange` false))

(event `OpenKeypadUI`
  (bind _returnvalue (`|CreateWidget` (`self.KeypadUIClass`) (`GameplayStatics.GetPlayerController` 0)))
  (bind _output_get (set `self.CurrentKeypadUI` _returnvalue))
  (`UserWidget.AddToViewport` _output_get 0)
  (set `/Game/Blueprints/BP_Core/WBP_KeypadUI.OwnerKeypad` self (`self.CurrentKeypadUI`))
  (set `self.CurrentInput` "")
  ;[0.09133 0.06466 0.15 0.5] Display Update
  (`/Game/Blueprints/BP_Core/WBP_KeypadUI.UpdateDisplay` (`self.CurrentKeypadUI`) "----")
  ;[0 0.15 0.07191 0.5] Open Keyborad UI / Mouse Cursor
  (set `PlayerController.bShowMouseCursor` true (`GameplayStatics.GetPlayerController` 0))
  (`WidgetBlueprintLibrary.SetInputMode_UIOnlyEx` (`GameplayStatics.GetPlayerController` 0) (`self.CurrentKeypadUI`))
  (`self.DisableInput` (`GameplayStatics.GetPlayerCharacter` 0) (`GameplayStatics.GetPlayerController` 0)))

(event `CloseKeypadUI`
  ;[0.15 0 0.03003 0.5] UI Close
  (`Widget.RemoveFromParent` (`self.CurrentKeypadUI`))
  (set `self.CurrentInput` "")
  (set `PlayerController.bShowMouseCursor` false (`GameplayStatics.GetPlayerController` 0))
  (`WidgetBlueprintLibrary.SetInputMode_GameOnly` (`GameplayStatics.GetPlayerController` 0))
  (`self.EnableInput` (`GameplayStatics.GetPlayerCharacter` 0) (`GameplayStatics.GetPlayerController` 0))
  (set `self.CurrentKeypadUI` null))

(event `AppendDigit`
  (params (Digit :type String))
  ;[0.05367 0.15 0.1458 0.5] KeypadUI Input
  (if (< (`KismetStringLibrary.Len` (`self.CurrentInput`)) 4)
    (set `self.CurrentInput` (`KismetStringLibrary.Concat_StrStr` (`self.CurrentInput`) Digit))
    (`/Game/Blueprints/BP_Core/WBP_KeypadUI.UpdateDisplay` (`self.CurrentKeypadUI`) (`KismetTextLibrary.Conv_StringToText` (`self.CurrentInput`)))))

(event `ClearInput`
  ;[0.04759 0.15 0.01432 0.5] ClearInput
  (set `self.CurrentInput` "")
  (`/Game/Blueprints/BP_Core/WBP_KeypadUI.UpdateDisplay` (`self.CurrentKeypadUI`) "----"))

(event `SubmitCode`
  ;[0.1484 0.02486 0.15 0.5] Submit
  (if (`KismetStringLibrary.EqualEqual_StrStr` (`self.CurrentInput`) (`self.CorrectCode`))
    (`/Game/Blueprints/BP_Core/BP_KeypadDoor.OpenDoorFromKeypad` (`self.LinkedDoor`))
    (`self.CloseKeypadUI`)
    (else
      (`/Game/Blueprints/BP_Core/WBP_KeypadUI.UpdateDisplay` (`self.CurrentKeypadUI`) "ERROR")
      (`KismetSystemLibrary.Delay` 0.8)
      (set `self.CurrentInput` "")
      (`/Game/Blueprints/BP_Core/WBP_KeypadUI.UpdateDisplay` (`self.CurrentKeypadUI`) "----"))))

(fn `UserConstructionScript`)