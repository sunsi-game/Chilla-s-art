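; Keypad door actor that swings open when its OpenDoorFromKeypad event is called, then closes itself automatically.
; Opening and closing each toggle IsDoor behind an EnableDoor check, play a wood door sound, and drive door yaw through separate timelines, hiding the icon and updating IsDoorOpen.
; A six-second Delay on the opening timeline's update triggers CloseDoorAuto.
; The Interaction event is empty, and an older FlipFlop toggle is left unconnected.
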(event `self.Interaction`
  ;[0 0.024 0.1] Open and Close DOOR
)

(event `OpenDoorFromKeypad`
  ;[0.15 0.1314 0.06724 0.5] OpenDoor
  (if (`self.bEnableDoor`)
    (bind _output_get (set `self.IsDoor` (!= (`self.IsDoor`) true)))
    (if _output_get
      (`GameplayStatics.PlaySoundAtLocation` "/Game/SmallSoundKit/SSKWav/DoorsWav/Drs_Wood_Door_Open_01.Drs_Wood_Door_Open_01" (`self.K2_GetActorLocation`) (struct) 1.0 1.0 0.0 null null null null)
      (bind (_direction _open___close_door) (`Timeline|Timeline` :!via `PlayFromStart`)
        (:`Update`
          (`SceneComponent.K2_SetRelativeRotation` (`self.Door`) (`KismetMathLibrary.MakeRotator` 0.0 0.0 (`KismetMathLibrary.Lerp` -90.0 -190.0 _open___close_door)) false false)
          (`SceneComponent.SetVisibility` (`self.Icon`) false false)
          (set `self.Is Door Open?` true)
          (`KismetSystemLibrary.Delay` 6.0)
          (`self.CloseDoorAuto`))))))

(event `CloseDoorAuto`
  (if (`self.bEnableDoor`)
    (bind _output_get (set `self.IsDoor` (!= (`self.IsDoor`) true)))
    (if (not _output_get)
      (`GameplayStatics.PlaySoundAtLocation` "/Game/SmallSoundKit/SSKWav/DoorsWav/Drs_Wood_Door_Close_01.Drs_Wood_Door_Close_01" (`self.K2_GetActorLocation`) (struct) 1.0 1.0 0.0 null null null null)
      (bind (_direction _open___close_door) (`Timeline|Timeline_0` :!via `ReverseFromEnd`)
        (:`Update`
          (`SceneComponent.K2_SetRelativeRotation` (`self.Door`) (`KismetMathLibrary.MakeRotator` 0.0 0.0 (`KismetMathLibrary.Lerp` -90.0 -190.0 _open___close_door)) false false)
          (`SceneComponent.SetVisibility` (`self.Icon`) false false)
          (set `self.Is Door Open?` false))))))

(fn `UserConstructionScript`)