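; BP_Paper1 is an interactable paper note actor that shows a hint reading "0 X X X" on screen.
; On Interaction it creates a WBP_PaperViewer widget with a reference to itself, sets the note text and adds it to the viewport.
; A NoteOpen flag blocks duplicate viewers until the NoteOpenclose event resets it.
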(event `self.Interaction`
  (if (not (`self.bNoteOpen`))
    (bind _returnvalue (`|CreateWidget` "/Game/Blueprints/BP_Core/WBP_PaperViewer.WBP_PaperViewer_C" (`GameplayStatics.GetPlayerController` 0) self))
    (bind _output_get (set `self.NoteViewerRef` _returnvalue))
    (`/Game/Blueprints/BP_Core/WBP_PaperViewer.SetNoteText` _output_get "0 X X X")
    (`UserWidget.AddToViewport` (`self.NoteViewerRef`) 0)
    (set `self.bNoteOpen` true)))

(event `Note Open close`
  (set `self.bNoteOpen` false))

(fn `UserConstructionScript`)