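; BP_TePo is an actor that jumps straight up to a fixed world height when its Fly event is called.
; Fly keeps the current X and Y, sets Z without sweeping and plays the Po sound at 1.5 times volume.
; An unconnected, never-executed branch holds descent logic gated by FlyAway, using a short downward trace to stop; Tick and construction are empty.
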(event `self.ReceiveTick`
  (params (DeltaSeconds :type "Float (single-precision)")))

(event `Fly`
  (`self.K2_SetActorLocation` (`KismetMathLibrary.MakeVector` (.x (`self.K2_GetActorLocation`)) (.y (`self.K2_GetActorLocation`)) 2800.0))
  (`GameplayStatics.PlaySoundAtLocation` "/Game/BP_Level/Sounds/po.po" (0.0 0.0 0.0) (struct) 1.5 1.0 0.0 null null null null))

(fn `UserConstructionScript`)