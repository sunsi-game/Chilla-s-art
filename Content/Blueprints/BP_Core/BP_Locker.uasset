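; BP_Locker is a locker with a drawer that toggles open and closed through an Interaction event.
; BeginPlay caches the drawer's closed relative location and derives the open one from a fixed local Y offset.
; A timeline plays or reverses on each interaction, lerping the drawer mesh between the two positions.
; An interaction box tracks whether the third-person character is in range, though the Interaction event does not check that flag.
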(event `self.ReceiveBeginPlay`
  ; Closed Location Saved
  (set `self.ClosedLocation` (`SceneComponent.RelativeLocation` (`self.DrawerMesh`)))
  (set `self.OpenedLocation` (+ (`self.ClosedLocation`) (`KismetMathLibrary.MakeVector` 0.0 40.0))))

(event `/Game/Horror_Template/Blueprinnts/Interfaces/Interaction_Interface/BPI_Interaction.Interaction`
  (if (`self.bIsOpened`)
    (set `self.bIsOpened` false)
    (bind (_direction _alpha) (`Timeline|TL_DrawerOpen` :!via `Reverse` :!label _label)
      (:`Update`
        (`SceneComponent.K2_SetRelativeLocation` (`self.DrawerMesh`) (`KismetMathLibrary.VLerp` (`self.ClosedLocation`) (`self.OpenedLocation`) _alpha) false false)))
    (else
      (set `self.bIsOpened` true)
      (goto _label))))

(event `self.InteractionBox.OnComponentBeginOverlap`
  (params (OverlappedComponent :type "PrimitiveComponent Object Reference") (OtherActor :type "Actor Object Reference") (OtherComp :type "PrimitiveComponent Object Reference") (OtherBodyIndex :type Integer) (bFromSweep :type Boolean) (SweepResult :type "HitResult Structure (by ref)"))
  (cast `/Game/Horror_Template/Blueprinnts/BP_ThirdPersonCharacter` OtherActor)
  (set `self.bPlayerInRange` true))

(event `self.InteractionBox.OnComponentEndOverlap`
  (params (OverlappedComponent :type "PrimitiveComponent Object Reference") (OtherActor :type "Actor Object Reference") (OtherComp :type "PrimitiveComponent Object Reference") (OtherBodyIndex :type Integer))
  (cast `/Game/Horror_Template/Blueprinnts/BP_ThirdPersonCharacter` OtherActor)
  (set `self.bPlayerInRange` false))

(fn `UserConstructionScript`)