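; Bed trigger that plays a scripted bedtime phone-call cutscene when BP_ThirdPersonCharacter overlaps InteractionBox.
; It flags the character as in sequence, locks input, turns off the flashlight and snaps the player into a fixed pose.
; A chain of Delays times voiced Korean messages via BP_MessageDirector, call sounds and the smartphone reveal.
; It ends by adding a fade-out widget, teleporting the player to another location and restoring input.
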(event `self.InteractionBox.OnComponentBeginOverlap`
  (params (OverlappedComponent :type "PrimitiveComponent Object Reference") (OtherActor :type "Actor Object Reference") (OtherComp :type "PrimitiveComponent Object Reference") (OtherBodyIndex :type Integer) (bFromSweep :type Boolean) (SweepResult :type "HitResult Structure (by ref)"))
  ;[0.15 0.1449 0.02947 0.5] Position
  (bind _asbp_third_person_character (cast `/Game/Horror_Template/Blueprinnts/BP_ThirdPersonCharacter` OtherActor))
  (set `/Game/Horror_Template/Blueprinnts/BP_ThirdPersonCharacter.IsInSequence` true _asbp_third_person_character)
  (`Controller.SetIgnoreLookInput` (`GameplayStatics.GetPlayerController` 0) true)
  (`Controller.SetIgnoreMoveInput` (`GameplayStatics.GetPlayerController` 0) true)
  (bind _asbp_third_person_character_2 (cast `/Game/Horror_Template/Blueprinnts/BP_ThirdPersonCharacter` OtherActor))
  (`/Game/Horror_Template/Blueprinnts/BP_ThirdPersonCharacter.TrunOffFlashlight` _asbp_third_person_character_2)
  (`self.K2_SetActorLocation` (`GameplayStatics.GetPlayerCharacter` 0) (-490.0 -4600.0 120.0) false false)
  (`Controller.SetControlRotation` (`GameplayStatics.GetPlayerController` 0) (`KismetMathLibrary.MakeRotator` 0.0 0.0 89.0))
  (`self.K2_SetActorRotation` (`GameplayStatics.GetPlayerCharacter` 0) (struct :`Yaw` 89.0) false)
  ;[0.15 0 0.06211 0.5] Voice
  (bind _returnvalue (`GameplayStatics.GetActorOfClass` "/Game/BP_Level/UI/BP_MessageDirector.BP_MessageDirector_C"))
  (`/Game/BP_Level/UI/BP_MessageDirector.PlayMessageWithVoice` _returnvalue "오늘은 너무 피곤하네… 빨리 자야겠어." "/Game/BP_Level/Voices/Badroom1.Badroom1" false)
  (`KismetSystemLibrary.Delay` 5.0)
  (`GameplayStatics.PlaySound2D` "/Game/BP_Level/Voices/ball.ball" 1.0 1.0 0.0 null null)
  (`KismetSystemLibrary.Delay` 2.5)
  (`self.SetActorHiddenInGame` (`self.bSmartPhone`) false)
  (bind _returnvalue_2 (`GameplayStatics.GetActorOfClass` "/Game/BP_Level/UI/BP_MessageDirector.BP_MessageDirector_C"))
  (`/Game/BP_Level/UI/BP_MessageDirector.PlayMessageWithVoice` _returnvalue_2 "여보세요?." "/Game/BP_Level/Voices/もしもし……？.もしもし……？" false)
  (`KismetSystemLibrary.Delay` 3.5)
  (bind _returnvalue_3 (`GameplayStatics.GetActorOfClass` "/Game/BP_Level/UI/BP_MessageDirector.BP_MessageDirector_C"))
  (`/Game/BP_Level/UI/BP_MessageDirector.PlayMessageWithVoice` _returnvalue_3 "지금 집에 있지?" "/Game/BP_Level/Voices/01？.01？" false)
  (`KismetSystemLibrary.Delay` 4.0)
  (bind _returnvalue_4 (`GameplayStatics.GetActorOfClass` "/Game/BP_Level/UI/BP_MessageDirector.BP_MessageDirector_C"))
  (`/Game/BP_Level/UI/BP_MessageDirector.PlayMessageWithVoice` _returnvalue_4 "잠깐만!!!" "/Game/BP_Level/Voices/02。.02。" false)
  (`KismetSystemLibrary.Delay` 2.5)
  (`GameplayStatics.PlaySound2D` "/Game/BP_Level/Voices/call_end.call_end" 1.0 1.0 0.0 null null)
  (`KismetSystemLibrary.Delay` 3.5)
  (bind _returnvalue_5 (`GameplayStatics.GetActorOfClass` "/Game/BP_Level/UI/BP_MessageDirector.BP_MessageDirector_C"))
  (`/Game/BP_Level/UI/BP_MessageDirector.PlayMessageWithVoice` _returnvalue_5 "방금 뭐였지??" "/Game/BP_Level/Voices/nasi……？.nasi……？" false)
  (`KismetSystemLibrary.Delay` 3.0)
  (bind _returnvalue_6 (`GameplayStatics.GetActorOfClass` "/Game/BP_Level/UI/BP_MessageDirector.BP_MessageDirector_C"))
  (`/Game/BP_Level/UI/BP_MessageDirector.PlayMessageWithVoice` _returnvalue_6 "먼저 그 애 집부터 가보자..." "/Game/BP_Level/Voices/nasi2.nasi2" false)
  (`KismetSystemLibrary.Delay` 4.0)
  (bind _returnvalue_7 (`|CreateWidget` "/Game/Blueprints/WBP_Fade_OUT.WBP_Fade_OUT_C" (`GameplayStatics.GetPlayerController` 0)))
  (bind _output_get (set `self.Fade Out UI` _returnvalue_7))
  (`UserWidget.AddToViewport` _output_get 0)
  (`self.K2_SetActorLocation` (`GameplayStatics.GetPlayerCharacter` 0) (-589.37687 387.574457 3016.737459) false false)
  (`Controller.SetIgnoreLookInput` (`GameplayStatics.GetPlayerController` 0) false)
  (`Controller.SetIgnoreMoveInput` (`GameplayStatics.GetPlayerController` 0) false)
  (`Controller.SetControlRotation` (`GameplayStatics.GetPlayerController` 0) (`KismetMathLibrary.MakeRotator` 0.0 0.0 270.0))
  (`self.K2_SetActorRotation` (`GameplayStatics.GetPlayerCharacter` 0) (struct :`Yaw` 270.0) false))

(fn `UserConstructionScript`)