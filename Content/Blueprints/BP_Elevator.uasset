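; BP_Elevator is an elevator actor that plays a one-shot animation when interacted with while the player is in range.
; A Box trigger tracks whether BP_ThirdPersonCharacter is inside, gating the Interaction event.
; Interaction turns off Box1 collision, plays the animation, then restores collision after a fixed delay timed in seconds.
; An IsPlaying flag blocks retriggering until that delay ends.
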(event `self.Box.OnComponentBeginOverlap`
  (params (OverlappedComponent :type "PrimitiveComponent Object Reference") (OtherActor :type "Actor Object Reference") (OtherComp :type "PrimitiveComponent Object Reference") (OtherBodyIndex :type Integer) (bFromSweep :type Boolean) (SweepResult :type "HitResult Structure (by ref)"))
  (cast `/Game/Horror_Template/Blueprinnts/BP_ThirdPersonCharacter` OtherActor)
  (set `self.bPlayerInRange` true))

(event `self.Box.OnComponentEndOverlap`
  (params (OverlappedComponent :type "PrimitiveComponent Object Reference") (OtherActor :type "Actor Object Reference") (OtherComp :type "PrimitiveComponent Object Reference") (OtherBodyIndex :type Integer))
  (cast `/Game/Horror_Template/Blueprinnts/BP_ThirdPersonCharacter` OtherActor)
  (set `self.bPlayerInRange` false))

(event `/Game/Horror_Template/Blueprinnts/Interfaces/Interaction_Interface/BPI_Interaction.Interaction`
  (if (`self.bPlayerInRange`)
    (if (not (`self.bIsPlaying`))
      (set `self.bIsPlaying` true)
      (`PrimitiveComponent.SetCollisionEnabled` (`self.Box1`) "NoCollision")
      (`SkeletalMeshComponent.PlayAnimation` (`self.Elevator`) "/Game/Fab/download/Elevator/ElevatorAnimation_Anim.ElevatorAnimation_Anim" false)
      (`KismetSystemLibrary.Delay` 11.5)
      (`PrimitiveComponent.SetCollisionEnabled` (`self.Box1`) "QueryAndPhysics")
      (set `self.bIsPlaying` false))))

(event `self.ReceiveBeginPlay`
  (`PrimitiveComponent.SetCollisionEnabled` (`self.Box1`) "QueryAndPhysics"))

(fn `UserConstructionScript`)